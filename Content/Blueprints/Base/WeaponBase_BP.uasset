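; Base weapon Blueprint that deals damage on overlap and can be equipped by the player.
; Sphere overlaps with actors other than the owner apply Damage and print it, throttled by a DoOnce that resets after a short delay.
; Activate and deactivate events switch Collision between an overlap-all profile and no collision.
; Interact sends an equip message to a Player-tagged actor and turns off mesh physics.
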(event `self.Sphere.OnComponentBeginOverlap`
  (params (OverlappedComponent :type "PrimitiveComponent Object Reference") (OtherActor :type "Actor Object Reference") (OtherComp :type "PrimitiveComponent Object Reference") (OtherBodyIndex :type Integer) (bFromSweep :type Boolean) (SweepResult :type "HitResult Structure (by ref)"))
  (bind _damage (`self.Damage`))
  (bind _output_get (set `self.Other Actor` OtherActor))
  (if (!= OtherActor (`self.GetOwner`))
    (`/Engine/EditorBlueprintResources/StandardMacros.DoOnce` false :!label _label
      (:`Completed`
        (`GameplayStatics.ApplyDamage` _output_get _damage)
        (`KismetSystemLibrary.PrintString` (`KismetStringLibrary.Conv_DoubleToString` _damage))
        (`KismetSystemLibrary.Delay` 0.5)
        (goto _label :!via `Reset`)))))

(event `WeaponActiv`
  (`PrimitiveComponent.SetCollisionProfileName` (`self.Collision`) "OverlapAll" true))

(event `WeaponDeactive`
  (`PrimitiveComponent.SetCollisionEnabled` (`self.Collision`) "NoCollision"))

(event `/Game/Blueprints/Interfaces/PlayerPickUP_INT.Interact`
  (if (`self.ActorHasTag` (`self.Other Actor`) "Player")
    (message `/Game/Blueprints/Interfaces/PlayerPickUP_INT.EquipWeapons` (`self.Other Actor`) self)
    (`PrimitiveComponent.SetSimulatePhysics` (`self.StaticMesh`) false)))

(fn `UserConstructionScript`)