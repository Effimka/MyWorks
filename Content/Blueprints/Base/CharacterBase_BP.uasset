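; Base player character Blueprint with camera-relative movement, HP and stamina-style SP, and a great sword hit reaction.
; Input axes drive look and yaw-only movement, while BeginPlay sets weapon ownership and creates the main HUD.
; Damage plays an impact montage or, at zero HP, a one-time death animation that then freezes and disables movement.
; Tick pushes stats to HealthStatsBP and regenerates SP through a Delay.
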(event `InputAxis|Turn`
  (params (AxisValue :type "Float (single-precision)"))
  ;[1 1 1] Comment
  (`self.AddControllerYawInput` AxisValue))

(event `InputAxis|MoveFB`
  (params (AxisValue :type "Float (single-precision)"))
  (bind (_returnvalue_roll _returnvalue_pitch _returnvalue_yaw) (`KismetMathLibrary.BreakRotator` (`self.GetControlRotation`)))
  ;[1 1 1] Movement
  (`self.AddMovementInput` (`KismetMathLibrary.GetForwardVector` (`KismetMathLibrary.MakeRotator` 0.0 0.0 _returnvalue_yaw)) AxisValue))

(event `InputAxis|LookUp`
  (params (AxisValue :type "Float (single-precision)"))
  ;[1 1 1] Comment
  (`self.AddControllerPitchInput` AxisValue))

(event `InputAxis|MoveLR`
  (params (AxisValue :type "Float (single-precision)"))
  (bind (_returnvalue_roll _returnvalue_pitch _returnvalue_yaw) (`KismetMathLibrary.BreakRotator` (`self.GetControlRotation`)))
  ;[1 1 1] Movement
  (`self.AddMovementInput` (`KismetMathLibrary.GetRightVector` (`KismetMathLibrary.MakeRotator` 0.0 0.0 _returnvalue_yaw)) AxisValue))

(event `self.ReceiveAnyDamage`
  (params (Damage :type "Float (single-precision)") (DamageType :type "DamageType Object Reference") (InstigatedBy :type "Controller Object Reference") (DamageCauser :type "Actor Object Reference"))
  (bind _output_get (set `self.CurrentHP` (- (`self.CurrentHP`) Damage)))
  (if (<= _output_get 0.0)
    (`/Engine/EditorBlueprintResources/StandardMacros.DoOnce` false
      (:`Completed`
        (`SkeletalMeshComponent.PlayAnimation` (`self.Mesh`) "/Game/Animation/Animation/IDLEWalkWithWeapon/Standing_Death_Left_02.Standing_Death_Left_02" false)
        (`KismetSystemLibrary.Delay` 2.0)
        (set `SkeletalMeshComponent.bPauseAnims` true (`self.Mesh`))
        (`CharacterMovementComponent.DisableMovement` (`self.CharacterMovement`))))
    (else
      (`self.PlayAnimMontage` "/Game/Animation/AnimMontage/Great_Sword_Impact_Montage.Great_Sword_Impact_Montage"))))

(event `self.ReceiveBeginPlay`
  (`|ExecutionSequence`
    (:`then_0`
      (`self.SetOwner` (`ChildActorComponent.ChildActor` (`self.Weapon`)) self))
    (:`then_1`
      (`/Game/Blueprints/Player/Blueprints/HealthStats_BP.SetHPandSP` (`self.HealthStats_BP`) (`self.MaxHP`) (`self.CurrentHP`) (`self.MaxSP`) (`self.CurrentSP`) :!label _label)
      (if (< (`self.CurrentSP`) (`self.MaxSP`))
        (`KismetSystemLibrary.Delay` 4.0)
        (set `self.CurrentSP` (+ (`self.CurrentSP`) 15.0))))
    (:`then_2`
      (bind _returnvalue (`|CreateWidget` "/Game/UI/Main_HUD.Main_HUD_C"))
      (`UserWidget.AddToViewport` _returnvalue 0))))

(event `self.ReceiveTick`
  (params (DeltaSeconds :type "Float (single-precision)"))
  (goto _label))

(fn `UserConstructionScript`)