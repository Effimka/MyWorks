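; Animation notify state that marks the damage window of a weapon attack within an animation.
; On begin and end, it casts the mesh owner to CharacterBase_BP and that character's Weapon child actor to WeaponBase_BP.
; It calls WeaponActiv on the weapon when the window opens and WeaponDeactive when it closes.
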(fn `Received_NotifyBegin`
  (params (MeshComp :type "SkeletalMeshComponent Object Reference") (Animation :type "AnimSequenceBase Object Reference") (TotalDuration :type "Float (double-precision)"))
  (returns (ReturnValue :type Boolean))
  (bind _ascharacter_base_bp (cast `/Game/Blueprints/Base/CharacterBase_BP` (`ActorComponent.GetOwner` MeshComp)))
  (bind _asweapon_base_bp (cast `/Game/Blueprints/Base/WeaponBase_BP` (`ChildActorComponent.ChildActor` (`/Game/Blueprints/Base/CharacterBase_BP.Weapon` _ascharacter_base_bp))))
  (`/Game/Blueprints/Base/WeaponBase_BP.WeaponActiv` _asweapon_base_bp)
  (return false))

(fn `Received_NotifyEnd`
  (params (MeshComp :type "SkeletalMeshComponent Object Reference") (Animation :type "AnimSequenceBase Object Reference"))
  (returns (ReturnValue :type Boolean))
  (bind _ascharacter_base_bp (cast `/Game/Blueprints/Base/CharacterBase_BP` (`ActorComponent.GetOwner` MeshComp)))
  (bind _asweapon_base_bp (cast `/Game/Blueprints/Base/WeaponBase_BP` (`ChildActorComponent.ChildActor` (`/Game/Blueprints/Base/CharacterBase_BP.Weapon` _ascharacter_base_bp))))
  (`/Game/Blueprints/Base/WeaponBase_BP.WeaponDeactive` _asweapon_base_bp)
  (return false))