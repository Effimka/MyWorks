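; Base enemy character that carries a socketed mesh, likely a weapon, and damages the player on contact.
; BeginPlay snaps the static mesh to the BattleSct socket, and PawnSensing forwards sightings to EnemyController_BP.
; Box overlaps with Player-tagged actors subtract fixed HP directly from Player_BP and play an impact montage on it.
; Tick polls CurrentHP and, at zero or below, repeatedly sets the static mesh to simulate physics with blocking collision.
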(event `self.ReceiveBeginPlay`
  (`parent.ReceiveBeginPlay`)
  (`SceneComponent.K2_AttachToComponent` (`self.StaticMesh`) (`self.Mesh`) "BattleSct" "SnapToTarget" "SnapToTarget" "SnapToTarget" true))

(event `self.ReceiveTick`
  (params (DeltaSeconds :type "Float (single-precision)"))
  (`parent.ReceiveTick` DeltaSeconds)
  (if (<= (`self.CurrentHP`) 0.0)
    (`PrimitiveComponent.SetSimulatePhysics` (`self.StaticMesh`) true)
    (`PrimitiveComponent.SetCollisionProfileName` (`self.StaticMesh`) "BlockAll" true)))

(event `self.Box.OnComponentBeginOverlap`
  (params (OverlappedComponent :type "PrimitiveComponent Object Reference") (OtherActor :type "Actor Object Reference") (OtherComp :type "PrimitiveComponent Object Reference") (OtherBodyIndex :type Integer) (bFromSweep :type Boolean) (SweepResult :type "HitResult Structure (by ref)"))
  (if (`self.ActorHasTag` OtherActor "Player")
    (bind _asplayer_bp (cast `/Game/Blueprints/Player/Blueprints/Player_BP` OtherActor))
    (set `/Game/Blueprints/Base/CharacterBase_BP.CurrentHP` (- (`/Game/Blueprints/Base/CharacterBase_BP.CurrentHP` _asplayer_bp) 15.0) _asplayer_bp)
    (`self.PlayAnimMontage` _asplayer_bp "/Game/Animation/AnimMontage/Great_Sword_Impact_Montage.Great_Sword_Impact_Montage" 1.0 "None")))

(event `self.PawnSensing.OnSeePawn`
  (params (Pawn :type "Pawn Object Reference"))
  (bind _asenemy_controller_bp (cast `/Game/Blueprints/enemy/Blueprints/Base/EnemyController_BP` (`self.GetController`)))
  (`/Game/Blueprints/enemy/Blueprints/Base/EnemyController_BP.OnSeePawn` _asenemy_controller_bp Pawn))

(fn `UserConstructionScript`
  (`parent.UserConstructionScript`))