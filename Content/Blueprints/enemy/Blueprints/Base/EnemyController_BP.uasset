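; AI controller for a melee enemy that patrols random reachable points until it sees the player, then moves in to attack.
; Attack turns to the player and plays random montages that spend SP, following two light attacks with a costlier heavy one that resets the combo.
; A short cooldown gates attacks, and each call restarts a timeline after a delay, though its update output drives nothing here.
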(event `Attack`
  (bind _as_enemy_bp (`self.As Enemy BP`))
  (bind _as_enemy_bp_2 (`self.As Enemy BP`))
  (bind _returnvalue (- (`/Game/Blueprints/Base/CharacterBase_BP.CurrentSP` (`self.As Enemy BP`)) 20.0))
  (bind _returnvalue_2 (- (`/Game/Blueprints/Base/CharacterBase_BP.CurrentSP` (`self.As Enemy BP`)) 40.0))
  (`self.K2_SetActorRotation` (`self.K2_GetPawn`) (`KismetMathLibrary.FindLookAtRotation` (`self.K2_GetActorLocation` (`self.K2_GetPawn`)) (`self.K2_GetActorLocation` (`self.As Player BP`))) false)
  (`|ExecutionSequence`
    (:`then_0`
      (if (`self.CanAttack`)
        (if (> (`/Game/Blueprints/Base/CharacterBase_BP.CurrentSP` (`self.As Enemy BP`)) 0.0)
          (if (>= (`self.AttackCount`) 2)
            (if (not (< (`/Game/Blueprints/Base/CharacterBase_BP.CurrentSP` (`self.As Enemy BP`)) 50.0))
              (switch `int` (`KismetMathLibrary.RandomIntegerInRange` 0 2)
                (:`0`
                  (set `/Game/Blueprints/Base/CharacterBase_BP.CurrentSP` _returnvalue_2 _as_enemy_bp)
                  (`Character.PlayAnimMontage` _as_enemy_bp "/Game/Animation/AnimMontage/Standing_Melee_Attack_360_Low_Montage.Standing_Melee_Attack_360_Low_Montage" 1.0 "None")
                  (`self.ResetKick`))
                (:`1`
                  (set `/Game/Blueprints/Base/CharacterBase_BP.CurrentSP` _returnvalue_2 _as_enemy_bp)
                  (`Character.PlayAnimMontage` _as_enemy_bp "/Game/Animation/AnimMontage/Standing_Melee_Attack_Backhand_Montage.Standing_Melee_Attack_Backhand_Montage" 1.0 "None")
                  (`self.ResetKick`))
                (:`2`
                  (set `/Game/Blueprints/Base/CharacterBase_BP.CurrentSP` _returnvalue_2 _as_enemy_bp)
                  (`Character.PlayAnimMontage` _as_enemy_bp "/Game/Animation/AnimMontage/Great_Sword_Slash_Montage.Great_Sword_Slash_Montage" 1.0 "None")
                  (`self.ResetKick`)))
              (set `self.CanAttack` false :!label _label)
              (`|ExecutionSequence`
                (:`then_0`
                  (`KismetSystemLibrary.Delay` 0.4)
                  (set `self.CanAttack` true))
                (:`then_1`
                  (`Timeline|Timeline_0` :!via `Stop` :!label _label_2))))
            (else
              (switch `int` (`KismetMathLibrary.RandomIntegerInRange` 0 2)
                (:`0`
                  (set `/Game/Blueprints/Base/CharacterBase_BP.CurrentSP` _returnvalue _as_enemy_bp_2)
                  (`Character.PlayAnimMontage` _as_enemy_bp_2 "/Game/Animation/AnimMontage/Standing_Melee_Attack_Downward_Montage.Standing_Melee_Attack_Downward_Montage" 1.0 "None"))
                (:`1`
                  (set `/Game/Blueprints/Base/CharacterBase_BP.CurrentSP` _returnvalue _as_enemy_bp_2)
                  (`Character.PlayAnimMontage` _as_enemy_bp_2 "/Game/Animation/AnimMontage/Stable_Sword_Inward_Slash_Montage.Stable_Sword_Inward_Slash_Montage" 1.0 "None"))
                (:`2`
                  (set `/Game/Blueprints/Base/CharacterBase_BP.CurrentSP` _returnvalue _as_enemy_bp_2)
                  (`Character.PlayAnimMontage` _as_enemy_bp_2 "/Game/Animation/AnimMontage/Great_Sword_Attack_Montage.Great_Sword_Attack_Montage" 1.0 "None")))
              (`/Engine/EditorBlueprintResources/StandardMacros.IncrementInt` (`self.AttackCount`)
                (:`  `
                  (goto _label))))))))
    (:`then_1`
      (`KismetSystemLibrary.Delay` 0.4)
      (goto _label_2 :!via `PlayFromStart`))))

(event `OnSeePawn`
  (params (Pawn :type "Pawn Object Reference"))
  (bind _asplayer_bp (cast `/Game/Blueprints/Player/Blueprints/Player_BP` Pawn))
  (bind _output_get (set `self.As Player BP` _asplayer_bp))
  (`|AIMoveTo` (`self.K2_GetPawn`) (0.0 0.0 0.0) _output_get 75.0
    (:`OnSuccess`
      (`self.Attack`))))

(event `self.ReceiveBeginPlay`
  (`self.Patrol`)
  (bind _asenemy_bp (cast `/Game/Blueprints/enemy/Blueprints/Base/Enemy_BP` (`self.K2_GetPawn`)))
  (set `self.As Enemy BP` _asenemy_bp))

(event `Patrol`
  (`/Engine/EditorBlueprintResources/StandardMacros.IsValid` (`self.As Player BP`)
    (:`Is Not Valid`
      (`|AIMoveTo` (`self.K2_GetPawn`) (`NavigationSystemV1.K2_GetRandomReachablePointInRadius` (`self.K2_GetActorLocation` (`self.K2_GetPawn`)) 1000.0 null null) null 150.0
        (:`OnSuccess`
          _)
        (:`OnFail`
          _))
      (`KismetSystemLibrary.Delay` 2.0)
      (`self.Patrol`))))

(fn `ResetKick`
  (set `self.AttackCount` 0))

(fn `UserConstructionScript`)