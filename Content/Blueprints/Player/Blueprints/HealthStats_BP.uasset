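; Player stats Blueprint that stores current and maximum HP and SP values.
; SetHPandSP overwrites all four values directly, without clamping or validation.
; GetStatsForHUD supplies the HUD with those values as truncated integer text, plus normalized HP and SP fractions for progress bars.
; The event graph holds no active logic, so the Blueprint acts purely as a data holder and formatter.
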(fn `GetStatsForHUD`
  (returns (MaxHP :type Text) (CurrentHP :type Text) (HPprogerssBar :type "Float (double-precision)") (MaxSP :type Text) (CurrentSP :type Text) (SPprogressBar :type "Float (double-precision)"))
  (return (`KismetTextLibrary.Conv_IntToText` (`KismetMathLibrary.FTrunc` (`self.MaxHP`))) (`KismetTextLibrary.Conv_IntToText` (`KismetMathLibrary.FTrunc` (`self.CurrentHP`))) (`KismetMathLibrary.NormalizeToRange` (`self.CurrentHP`) 0.0 (`self.MaxHP`)) (`KismetTextLibrary.Conv_IntToText` (`KismetMathLibrary.FTrunc` (`self.MaxSP`))) (`KismetTextLibrary.Conv_IntToText` (`KismetMathLibrary.FTrunc` (`self.CurrentSP`))) (`KismetMathLibrary.NormalizeToRange` (`self.CurrentSP`) 0.0 (`self.MaxSP`))))

(fn `SetHPandSP`
  (params (SetMaxHP :type "Float (double-precision)") (SetCurrentHP :type "Float (double-precision)") (SetMaxSP :type "Float (double-precision)") (SetCurrentSP :type "Float (double-precision)"))
  (set `self.MaxHP` SetMaxHP)
  (set `self.CurrentHP` SetCurrentHP)
  (set `self.MaxSP` SetMaxSP)
  (set `self.CurrentSP` SetCurrentSP))