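; Player character Blueprint handling melee combat, weapon equipping, interaction and death.
; Equip input toggles battle mode with montages, swapping anim classes; Equip/UnEquip events move the picked-up weapon between battle and shoulder sockets.
; Attacks spend stamina on random montages, switching to costlier ones after two hits; a timeline started on release resets the combo.
; Capsule overlaps gate interaction messages; a one-shot BeginPlay timer checks HP for death.
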(event `self.ReceiveBeginPlay`
  (`KismetSystemLibrary.K2_SetTimerDelegate` (delegate `Die`) 0.5))

(event `Die`
  (if (<= (`self.CurrentHP`) 0.0)
    (`/Engine/EditorBlueprintResources/StandardMacros.DoOnce` false
      (:`Completed`
        (`SkeletalMeshComponent.PlayAnimation` (`self.Mesh`) "/Game/Animation/Animation/IDLEWalkWithWeapon/Standing_Death_Left_02.Standing_Death_Left_02" false)
        (`KismetSystemLibrary.Delay` 2.0)
        (set `SkeletalMeshComponent.bPauseAnims` true (`self.Mesh`))
        (`CharacterMovementComponent.DisableMovement` (`self.CharacterMovement`))))))

(event `Equip`
  ;[1 1 1] EquipWeaponChangeMode
  (`self.K2_AttachToComponent` (`self.Weapon_0`) (`self.Mesh`) "BattleSct" "SnapToTarget" "SnapToTarget" "SnapToTarget" true))

(event `InputAction|Equip`
  (params (Key :type "Key Structure"))
  (bind _mesh (`self.Mesh`))
  ;[1 1 1] EquipWeaponChangeMode
  (:`Pressed`
    (if (`self.HaveWeapon`)
      (if (`self.BattleMod`)
        (bind _returnvalue (`self.PlayAnimMontage` "/Game/Animation/AnimMontage/UnEquip_Montage.UnEquip_Montage"))
        (set `self.BattleMod` false)
        (`KismetSystemLibrary.Delay` _returnvalue)
        (`SkeletalMeshComponent.SetAnimInstanceClass` _mesh "/Game/Animation/AnimBP/Animation_BP.Animation_BP_C")
        (else
          (bind _returnvalue_2 (`self.PlayAnimMontage` "/Game/Animation/AnimMontage/Equip_Montage.Equip_Montage"))
          (set `self.BattleMod` true)
          (`KismetSystemLibrary.Delay` _returnvalue_2)
          (`SkeletalMeshComponent.SetAnimInstanceClass` _mesh "/Game/Animation/AnimBP/FightAnim_BP.FightAnim_BP_C")
          (set `self.CanAttack` true))))))

(event `UnEquip`
  ;[1 1 1] EquipWeaponChangeMode
  (`self.K2_AttachToComponent` (`self.Weapon_0`) (`self.Mesh`) "LeftShoulderSct" "SnapToTarget" "SnapToTarget" "SnapToTarget" true))

(event `/Game/Blueprints/Interfaces/PlayerPickUP_INT.EquipWeapons`
  (params (Weapon :type "/Game/Blueprints/Base/WeaponBase_BP Object Reference"))
  ;[1 1 1] PickUpWeapons
  (bind _output_get (set `self.Weapon_0` Weapon))
  (if (not (`self.HaveWeapon`))
    (`self.K2_AttachToComponent` _output_get (`self.Mesh`) "LeftShoulderSct" "SnapToTarget" "SnapToTarget" "SnapToTarget" true)
    (set `self.HaveWeapon` true)))

(event `InputAction|Interact`
  (params (Key :type "Key Structure"))
  ;[1 1 1] Interact
  (:`Pressed`
    (if (`self.IsInteractedLocked`)
      (message `/Game/Blueprints/Interfaces/PlayerPickUP_INT.Interact` (`self.LastInterectActor`))
      (else
        (`/Engine/EditorBlueprintResources/StandardMacros.Gate` true :!label _label
          (:`Exit`
            (bind _output_get (set `self.LastInterectActor` (stale `self.CapsuleComponent.OnComponentBeginOverlap` OtherActor)))
            (message `/Game/Blueprints/Interfaces/PlayerPickUP_INT.Interact` _output_get)))))))

(event `self.CapsuleComponent.OnComponentBeginOverlap`
  (params (OverlappedComponent :type "PrimitiveComponent Object Reference") (OtherActor :type "Actor Object Reference") (OtherComp :type "PrimitiveComponent Object Reference") (OtherBodyIndex :type Integer) (bFromSweep :type Boolean) (SweepResult :type "HitResult Structure (by ref)"))
  ;[1 1 1] Interact
  (goto _label :!via `Open`))

(event `self.CapsuleComponent.OnComponentEndOverlap`
  (params (OverlappedComponent :type "PrimitiveComponent Object Reference") (OtherActor :type "Actor Object Reference") (OtherComp :type "PrimitiveComponent Object Reference") (OtherBodyIndex :type Integer))
  ;[1 1 1] Interact
  (goto _label :!via `Close`))

(event `InputAction|AttackButton`
  (params (Key :type "Key Structure"))
  (bind _returnvalue (- (`self.CurrentSP`) 20.0))
  (bind _returnvalue_2 (- (`self.CurrentSP`) 40.0))
  (:`Pressed`
    (if (`self.CanAttack`)
      (if (> (`self.CurrentSP`) 0.0)
        (if (>= (`self.AttackCount`) 2)
          (if (not (< (`self.CurrentSP`) 50.0))
            (switch `int` (`KismetMathLibrary.RandomIntegerInRange` 0 2)
              (:`0`
                (set `self.CurrentSP` _returnvalue_2)
                (`self.PlayAnimMontage` "/Game/Animation/AnimMontage/Standing_Melee_Attack_360_Low_Montage.Standing_Melee_Attack_360_Low_Montage")
                (`self.ResetKick`))
              (:`1`
                (set `self.CurrentSP` _returnvalue_2)
                (`self.PlayAnimMontage` "/Game/Animation/AnimMontage/Standing_Melee_Attack_Backhand_Montage.Standing_Melee_Attack_Backhand_Montage")
                (`self.ResetKick`))
              (:`2`
                (set `self.CurrentSP` _returnvalue_2)
                (`self.PlayAnimMontage` "/Game/Animation/AnimMontage/Great_Sword_Slash_Montage.Great_Sword_Slash_Montage")
                (`self.ResetKick`)))
            (set `self.CanAttack` false :!label _label_2)
            (`|ExecutionSequence`
              (:`then_0`
                (`KismetSystemLibrary.Delay` 0.4)
                (set `self.CanAttack` true))
              (:`then_1`
                (`Timeline|Timeline_0` :!via `Stop` :!label _label_3
                  (:`Finished`
                    (`self.ResetKick`))))))
          (else
            (switch `int` (`KismetMathLibrary.RandomIntegerInRange` 0 2)
              (:`0`
                (set `self.CurrentSP` _returnvalue)
                (`self.PlayAnimMontage` "/Game/Animation/AnimMontage/Standing_Melee_Attack_Downward_Montage.Standing_Melee_Attack_Downward_Montage")
                (`/Engine/EditorBlueprintResources/StandardMacros.IncrementInt` (`self.AttackCount`) :!label _label_4
                  (:`  `
                    (goto _label_2))))
              (:`1`
                (set `self.CurrentSP` _returnvalue)
                (`self.PlayAnimMontage` "/Game/Animation/AnimMontage/Stable_Sword_Inward_Slash_Montage.Stable_Sword_Inward_Slash_Montage")
                (goto _label_4))
              (:`2`
                (set `self.CurrentSP` _returnvalue)
                (`self.PlayAnimMontage` "/Game/Animation/AnimMontage/Great_Sword_Attack_Montage.Great_Sword_Attack_Montage"))))))))
  (:`Released`
    (goto _label_3 :!via `PlayFromStart`)))

(fn `ResetKick`
  (set `self.AttackCount` 0))

(fn `StopInteract`)

(fn `UserConstructionScript`
  (`parent.UserConstructionScript`))